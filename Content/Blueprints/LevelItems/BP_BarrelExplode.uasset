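; BP_BarrelExplode is an explosive barrel level item that blows up when its health runs out.
; Each SHealth health change briefly draws the value as debug text at the mesh.
; At zero or below, it applies an impulse to the mesh using its world location as the vector, fires the RadialForce impulse, spawns an enlarged explosion emitter, and destroys itself.
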(event OnHealthChanged(SHealth)
  (params (HealthComp :type S%20Health%20Component%20Object%20Reference) (Health :type Float%20%28single-precision%29) (HealthDelta :type Float%20%28single-precision%29) (DamageType :type Damage%20Type%20Object%20Reference) (InstigatedBy :type Controller%20Object%20Reference) (DamageCauser :type Actor%20Object%20Reference))
  (bind _staticmesh (Variables|Default|GetStaticMesh))
  (bind _returnvalue (Transformation|GetWorldLocation _staticmesh))
  (Rendering|Debug|DrawDebugString _returnvalue (Utilities|String|ToString(Float) Health) 0 "(R=1.000000,G=1.000000,B=1.000000,A=1.000000)" 0.5)
  (Math|Float|CompareFloat Health 0.0
    (:==
      _)
    (:<
      _))
  (Physics|AddImpulse (Variables|Default|GetStaticMesh) _returnvalue "None" false)
  (Class|RadialForceComponent|FireImpulse (Variables|Default|GetRadialForce))
  (Effects|SpawnEmitteratLocation "/Game/WeaponEffects/Explosion/P_Explosion.P_Explosion" _returnvalue "0, 0, 0" "5.000000,5.000000,5.000000")
  (Actor|DestroyActor))

(event EventBeginPlay)

(event Collision|EventActorBeginOverlap
  (params (OtherActor :type Actor%20Object%20Reference)))

(event EventTick
  (params (DeltaSeconds :type Float%20%28single-precision%29)))

(fn ConstructionScript)